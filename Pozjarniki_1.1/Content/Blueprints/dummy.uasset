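; A burning dummy actor that takes damage, with a big fire particle effect and a fire sound that reflect its health.
; Each hit lowers Health and scales the sound volume to it, and the fire deactivates once Health reaches zero.
; A Respawn event restores full Health, relights the fire and resets the volume, and both events print Health to the screen.
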(event Custom|Respawn
  (bind _output_get (Variables|Default|Sethealth 1e+02))
  (Development|PrintString (Utilities|String|ToString(Float) (Variables|Default|Gethealth)))
  (Variables|Default|Setisonfire true)
  (Components|Activation|Activate (Variables|Default|GetP_Fire_Big) false)
  (Audio|Components|Audio|SetVolumeMultiplier (Variables|Default|GetFire_sound) (/ _output_get 1e+02) :!class /Script/Engine.AudioComponent))

(event Game|Damage|EventAnyDamage
  (params (Damage :type Float%20%28single-precision%29) (DamageType :type Damage%20Type%20Object%20Reference) (InstigatedBy :type Controller%20Object%20Reference) (DamageCauser :type Actor%20Object%20Reference))
  (bind _output_get (Variables|Default|Sethealth (- (Variables|Default|Gethealth) Damage)))
  (Audio|Components|Audio|SetVolumeMultiplier (Variables|Default|GetFire_sound) (/ _output_get 1e+02) :!class /Script/Engine.AudioComponent)
  (if (<= _output_get 0.0)
    (Variables|Default|Setisonfire false)
    (else
      (Variables|Default|Setisonfire true)))
  (if (Variables|Default|Getisonfire)
    (Components|Activation|Activate (Variables|Default|GetP_Fire_Big) false)
    (else
      (Components|Activation|Deactivate (Variables|Default|GetP_Fire_Big))))
  (Development|PrintString (Utilities|String|ToString(Float) (Variables|Default|Gethealth))))

(fn ConstructionScript)