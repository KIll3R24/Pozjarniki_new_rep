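; First-person player character Blueprint handling movement, jumping, mouse look, interaction, hose-gun shooting and pausing.
; Interaction box-traces from the camera and messages the hit actor through BPI_interact or, failing that, BPI_read.
; Shooting requires EquippedGun, loops a montage timer and sends BPI_shooting messages to the BP_hose_fighting found by class.
; Gun pickup, marked unfinished, spawns and attaches that gun; pause opens a menu widget and pauses the game.
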(event Custom|Fire
  ;[1 1 1] Стрельба
  (if (Variables|Default|Getbisfire)
    (Animation|Montage|PlayMontage 0 "/Game/FP_from_UE/FirstPersonArms/Animations/FP_Rifle_Shoot_Montage.FP_Rifle_Shoot_Montage"
      (:then
        (Class|BPIShooting|Shooting(Message) (stale Input|ActionEvents|InputActionShoot _returnvalue) (Variables|Default|Getbisfire))))))

(event Custom|Gun_pickup
  ;[1 1 1] Подбор пушки (в процессе реализации)
  (bind _returnvalue (Game|SpawnActorfromClass "/Game/Blueprints/BP_hose_fighting.BP_hose_fighting_C" (Variables|Default|Getrifle) "Undefined" "MultiplyWithRoot" 0 0))
  (bind _output_get (Variables|Default|SetEquippedGun _returnvalue))
  (Transformation|AttachComponentToComponent _output_get (Variables|Default|GetGunLocation) "None" "SnapToTarget" "SnapToTarget" "KeepRelative" true))

(event Input|EnhancedActionEvents|EnhancedInputActionIA_Interaction
  (params (ActionValue :type Boolean) (ElapsedSeconds :type Float%20%28double-precision%29) (TriggeredSeconds :type Float%20%28double-precision%29) (InputAction :type Input%20Action%20Object%20Reference :default "/Game/Inputs/FirstPerson/Input/Actions/IA_Interaction.IA_Interaction"))
  ;[1 1 1] Interaction
  (:Started
    (bind _hitactor (Utilities|Trace))
    (if (Utilities|DoesObjectImplementInterface _hitactor "/Game/Blueprints/interfaces/BPI_interact.BPI_interact_C")
      (Class|BPIInteract|Interact(Message) _hitactor)
      (elif (Utilities|DoesObjectImplementInterface _hitactor "/Game/Blueprints/interfaces/BPI_read.BPI_read_C")
        (Variables|Default|Setisbookopened true)
        (Class|BPIRead|Read(Message) _hitactor)))))

(event Input|EnhancedActionEvents|EnhancedInputActionIA_Pause
  (params (ActionValue :type Boolean) (ElapsedSeconds :type Float%20%28double-precision%29) (TriggeredSeconds :type Float%20%28double-precision%29) (InputAction :type Input%20Action%20Object%20Reference :default "/Game/Inputs/FirstPerson/Input/Actions/IA_Pause.IA_Pause"))
  (bind _returnvalue (Game|GetPlayerController 0))
  ;[1 1 1] Пауза
  (if (not (Variables|Default|Getispausemenuopened))
    (Variables|Default|Setispausemenuopened true)
    (bind _returnvalue_2 (UserInterface|CreateWidget "/Game/Widgets/BP_FPUserPause.BP_FPUserPause_C" _returnvalue))
    (bind _output_get (Variables|Default|SetPause%20Menu%20Widget _returnvalue_2))
    (UserInterface|Viewport|AddtoViewport _output_get 0)
    (Input|SetInputModeGameandUI _returnvalue (Variables|Default|GetPause%20Menu%20Widget) "DoNotLock" true false)
    (bind _returnvalue_3 (Game|SetGamePaused true))
    (Variables|/Script/Engine.PlayerController|SetbShowMouseCursor _returnvalue _returnvalue_3)))

(event Input|EnhancedActionEvents|EnhancedInputActionIA_Jump
  (params (ActionValue :type Boolean) (ElapsedSeconds :type Float%20%28double-precision%29) (TriggeredSeconds :type Float%20%28double-precision%29) (InputAction :type Input%20Action%20Object%20Reference :default "/Game/Inputs/FirstPerson/Input/Actions/IA_Jump.IA_Jump"))
  ;[1 1 1] Прыжок
  (:Started
    (Character|Jump))
  (:Completed
    (Character|StopJumping)))

(event Input|ActionEvents|InputActionShoot
  (params (Key :type Key%20Structure :default "None"))
  ;[1 1 1] Стрельба
  (:Pressed
    (Variables|Default|Setbisfire true)
    (if (Utilities|IsValid (Variables|Default|GetEquippedGun))
      (Utilities|Time|SetTimerbyEvent (delegate Custom|Fire) 0.05 true)
      (bind _returnvalue (Actor|GetActorOfClass "/Game/Blueprints/BP_hose_fighting.BP_hose_fighting_C"))
      (if (Utilities|DoesObjectImplementInterface _returnvalue "/Game/Blueprints/interfaces/BPI_shooting.BPI_shooting_C")
        (Class|BPIShooting|Shooting(Message) _returnvalue (Variables|Default|Getbisfire)))))
  (:Released
    (Variables|Default|Setbisfire false)))

(event Input|AxisEvents|InputAxisMoveForward
  (params (AxisValue :type Float%20%28single-precision%29))
  ;[1 1 1] Движение по вертикали
  (Pawn|Input|AddMovementInput (Transformation|GetActorForwardVector) AxisValue false))

(event Input|AxisEvents|InputAxisLookHorizontal
  (params (AxisValue :type Float%20%28single-precision%29))
  ;[1 1 1] Поворот камеры горизонтальный
  (Pawn|Input|AddControllerYawInput AxisValue))

(event Input|AxisEvents|InputAxisLookVertical
  (params (AxisValue :type Float%20%28single-precision%29))
  ;[1 1 1] Поворот камеры вертикальный
  (Pawn|Input|AddControllerPitchInput (* AxisValue -1.0)))

(event Input|AxisEvents|InputAxisMoveRight
  (params (AxisValue :type Float%20%28single-precision%29))
  ;[1 1 1] Движение по горизонтали
  (Pawn|Input|AddMovementInput (Transformation|GetActorRightVector) AxisValue false))

(fn ConstructionScript)